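; Game Instance for a Town Clicker game that owns the persistent save game object.
; On Init it loads the ClickerSaveGame from a fixed slot, or creates and immediately saves a new one if none exists, and caches it in TCSaveGame.
; A SaveGame event writes the cached object back to that same slot.
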(event `self.ReceiveInit`
  (bind _returnvalue (`GameplayStatics.DoesSaveGameExist` (`self.gamesaveslot`)))
  (if _returnvalue
    (bind _returnvalue_2 (`GameplayStatics.LoadGameFromSlot` (`self.gamesaveslot`)))
    (bind _asclicker_save_game (cast `/Game/Blueprints/GameSave/ClickerSaveGame` _returnvalue_2))
    (set `self.TCSaveGame` _asclicker_save_game)
    (else
      (bind _returnvalue_3 (`GameplayStatics.CreateSaveGameObject` "/Game/Blueprints/GameSave/ClickerSaveGame.ClickerSaveGame_C"))
      (set `self.TCSaveGame` _returnvalue_3)
      (`GameplayStatics.SaveGameToSlot` (`self.TCSaveGame`) (`self.gamesaveslot`)))))

(event `SaveGame`
  (`GameplayStatics.SaveGameToSlot` (`self.TCSaveGame`) (`self.gamesaveslot`)))