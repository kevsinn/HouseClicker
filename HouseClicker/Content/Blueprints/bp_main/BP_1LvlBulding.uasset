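; Clickable, upgradeable house building for a money-tapping game, with one mesh component per level.
; A click or touch adds money to the WB_Main widget, plays a coin sound, spawns a Niagara effect and enables custom depth on all house meshes until release.
; Tick, after a short delay, reads the first building's upgrade count from that widget and swaps visibility to the matching level mesh.
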(event `self.Capsule.OnInputTouchBegin`
  (params (FingerIndex :type "ETouchIndex Enum" :default "Touch1") (TouchedComponent :type "PrimitiveComponent Object Reference"))
  ;[0 0 0 1 22] set render material
  (`PrimitiveComponent.SetRenderCustomDepth` (`self.1lvlHouse`) true :!label _label)
  (`PrimitiveComponent.SetRenderCustomDepth` (`self.2lvlHouse`) true)
  (`PrimitiveComponent.SetRenderCustomDepth` (`self.3lvlHouse`) true)
  (`PrimitiveComponent.SetRenderCustomDepth` (`self.4lvlHouse`) true)
  (`PrimitiveComponent.SetRenderCustomDepth` (`self.5lvlHouse`) true)
  (`PrimitiveComponent.SetRenderCustomDepth` (`self.6lvlHouse`) true)
  (`PrimitiveComponent.SetRenderCustomDepth` (`self.7lvlHouse`) true)
  (`PrimitiveComponent.SetRenderCustomDepth` (`self.8lvlHouse`) true)
  (`PrimitiveComponent.SetRenderCustomDepth` (`self.9lvlHouse`) true)
  (`PrimitiveComponent.SetRenderCustomDepth` (`self.10lvlHouse`) true)
  (`PrimitiveComponent.SetRenderCustomDepth` (`self.11lvlHouse`) true)
  (`PrimitiveComponent.SetRenderCustomDepth` (`self.12lvlHouse`) true)
  (`PrimitiveComponent.SetRenderCustomDepth` (`self.13lvlHouse`) true)
  (`PrimitiveComponent.SetRenderCustomDepth` (`self.14lvlHouse`) true)
  (`PrimitiveComponent.SetRenderCustomDepth` (`self.15lvlHouse`) true)
  (`PrimitiveComponent.SetRenderCustomDepth` (`self.16lvlHouse`) true)
  (`PrimitiveComponent.SetRenderCustomDepth` (`self.17lvlHouse`) true)
  (`PrimitiveComponent.SetRenderCustomDepth` (`self.18lvlHouse`) true)
  (set `self.IsInteracted` true)
  (bind _foundwidgets (`WidgetBlueprintLibrary.GetAllWidgetsOfClass` "/Game/Widgets/WB_Main.WB_Main_C" false))
  (bind _output_get (set `self.Found Widgets` _foundwidgets))
  (bind _output (`|GetArrayItem` _output_get))
  (set `/Game/Widgets/WB_Main.Money` (+ (`/Game/Widgets/WB_Main.Money` _output) 1.0) _output)
  (`AddComponent|NODE_AddNiagaraComponent-0` :`RelativeTransform` (`KismetMathLibrary.MakeTransform` (0.0 0.0 350.0) (struct :`Pitch` 100.0 :`Yaw` 100.0 :`Roll` 90.0)))
  (`GameplayStatics.PlaySoundAtLocation` "/Game/Sounds/cues/SC_Coins.SC_Coins" (`self.K2_GetActorLocation`) (struct) 1.0 1.0 0.0 null null null null))

(event `self.Capsule.OnClicked`
  (params (TouchedComponent :type "PrimitiveComponent Object Reference") (ButtonPressed :type "Key Structure"))
  (goto _label))

(event `self.Capsule.OnReleased`
  (params (TouchedComponent :type "PrimitiveComponent Object Reference") (ButtonReleased :type "Key Structure"))
  ;[0 0 0 1 22] set render material
  (`PrimitiveComponent.SetRenderCustomDepth` (`self.1lvlHouse`) false :!label _label_2)
  (`PrimitiveComponent.SetRenderCustomDepth` (`self.2lvlHouse`) false)
  (`PrimitiveComponent.SetRenderCustomDepth` (`self.3lvlHouse`) false)
  (`PrimitiveComponent.SetRenderCustomDepth` (`self.4lvlHouse`) false)
  (`PrimitiveComponent.SetRenderCustomDepth` (`self.5lvlHouse`) false)
  (`PrimitiveComponent.SetRenderCustomDepth` (`self.6lvlHouse`) false)
  (`PrimitiveComponent.SetRenderCustomDepth` (`self.7lvlHouse`) false)
  (`PrimitiveComponent.SetRenderCustomDepth` (`self.8lvlHouse`) false)
  (`PrimitiveComponent.SetRenderCustomDepth` (`self.9lvlHouse`) false)
  (`PrimitiveComponent.SetRenderCustomDepth` (`self.10lvlHouse`) false)
  (`PrimitiveComponent.SetRenderCustomDepth` (`self.11lvlHouse`) false)
  (`PrimitiveComponent.SetRenderCustomDepth` (`self.12lvlHouse`) false)
  (`PrimitiveComponent.SetRenderCustomDepth` (`self.13lvlHouse`) false)
  (`PrimitiveComponent.SetRenderCustomDepth` (`self.14lvlHouse`) false)
  (`PrimitiveComponent.SetRenderCustomDepth` (`self.15lvlHouse`) false)
  (`PrimitiveComponent.SetRenderCustomDepth` (`self.16lvlHouse`) false)
  (`PrimitiveComponent.SetRenderCustomDepth` (`self.17lvlHouse`) false)
  (`PrimitiveComponent.SetRenderCustomDepth` (`self.18lvlHouse`) false))

(event `self.Capsule.OnInputTouchEnd`
  (params (FingerIndex :type "ETouchIndex Enum" :default "Touch1") (TouchedComponent :type "PrimitiveComponent Object Reference"))
  (goto _label_2))

(event `self.ReceiveTick`
  (params (DeltaSeconds :type "Float (single-precision)"))
  (`KismetSystemLibrary.Delay` 0.1)
  ;[0 0 0 1 25] Upgrading and changing house mesh equal to its level
  (bind _foundwidgets (`WidgetBlueprintLibrary.GetAllWidgetsOfClass` "/Game/Widgets/WB_Main.WB_Main_C"))
  (bind _output_get (set `self.Found Widgets` _foundwidgets))
  (`|ExecutionSequence`
    (:`then_0`
      (bind ((`Upgrades_14_D8C4A89E4A9E31FA4A8E5B91E7EFABB6` _upgrades)) (break `/Game/Blueprints/structs/S_HouseInfo` (`|GetArrayItem` (`/Game/Widgets/WB_Main.Buldings` (`|GetArrayItem` _output_get)))))
      (if (== _upgrades 1)
        (`SceneComponent.SetVisibility` (`self.1lvlHouse`) false false)
        (`SceneComponent.SetVisibility` (`self.2lvlHouse`) true false)))
    (:`then_1`
      (if (== _upgrades 2)
        (`SceneComponent.SetVisibility` (`self.2lvlHouse`) false false)
        (`SceneComponent.SetVisibility` (`self.3lvlHouse`) true false)))
    (:`then_2`
      (if (== _upgrades 3)
        (`SceneComponent.SetVisibility` (`self.3lvlHouse`) false false)
        (`SceneComponent.SetVisibility` (`self.4lvlHouse`) true false)))
    (:`then_3`
      (if (== _upgrades 4)
        (`SceneComponent.SetVisibility` (`self.4lvlHouse`) false false)
        (`SceneComponent.SetVisibility` (`self.5lvlHouse`) true false)))
    (:`then_4`
      (if (== _upgrades 5)
        (`SceneComponent.SetVisibility` (`self.5lvlHouse`) false false)
        (`SceneComponent.SetVisibility` (`self.6lvlHouse`) true false)))
    (:`then_5`
      (if (== _upgrades 6)
        (`SceneComponent.SetVisibility` (`self.6lvlHouse`) false false)
        (`SceneComponent.SetVisibility` (`self.7lvlHouse`) true false)))
    (:`then_6`
      (if (== _upgrades 7)
        (`SceneComponent.SetVisibility` (`self.7lvlHouse`) false false)
        (`SceneComponent.SetVisibility` (`self.8lvlHouse`) true false)))
    (:`then_7`
      (if (== _upgrades 8)
        (`SceneComponent.SetVisibility` (`self.8lvlHouse`) false false)
        (`SceneComponent.SetVisibility` (`self.9lvlHouse`) true false)))
    (:`then_8`
      (if (== _upgrades 9)
        (`SceneComponent.SetVisibility` (`self.9lvlHouse`) false false)
        (`SceneComponent.SetVisibility` (`self.10lvlHouse`) true false)))
    (:`then_9`
      (if (== _upgrades 10)
        (`SceneComponent.SetVisibility` (`self.10lvlHouse`) false false)
        (`SceneComponent.SetVisibility` (`self.11lvlHouse`) true false)))
    (:`then_10`
      (if (== _upgrades 11)
        (`SceneComponent.SetVisibility` (`self.11lvlHouse`) false false)
        (`SceneComponent.SetVisibility` (`self.12lvlHouse`) true false)))
    (:`then_11`
      (if (== _upgrades 12)
        (`SceneComponent.SetVisibility` (`self.12lvlHouse`) false false)
        (`SceneComponent.SetVisibility` (`self.13lvlHouse`) true false)))
    (:`then_12`
      (if (== _upgrades 13)
        (`SceneComponent.SetVisibility` (`self.13lvlHouse`) false false)
        (`SceneComponent.SetVisibility` (`self.14lvlHouse`) true false)))
    (:`then_13`
      (if (== _upgrades 14)
        (`SceneComponent.SetVisibility` (`self.14lvlHouse`) false false)
        (`SceneComponent.SetVisibility` (`self.15lvlHouse`) true false)))
    (:`then_14`
      (if (== _upgrades 15)
        (`SceneComponent.SetVisibility` (`self.15lvlHouse`) false false)
        (`SceneComponent.SetVisibility` (`self.16lvlHouse`) true false)))
    (:`then_15`
      (if (== _upgrades 16)
        (`SceneComponent.SetVisibility` (`self.16lvlHouse`) false false)
        (`SceneComponent.SetVisibility` (`self.17lvlHouse`) true false)))
    (:`then_16`
      (if (== _upgrades 17)
        (`SceneComponent.SetVisibility` (`self.17lvlHouse`) false false)
        (`SceneComponent.SetVisibility` (`self.18lvlHouse`) true false)))))

(fn `UserConstructionScript`)