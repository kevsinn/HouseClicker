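; Clickable house building for a clicker game, with eighteen house level components.
; Clicking or touching its capsule enables custom depth on all houses, adds one Money to the first WB_Main widget found and spawns a Niagara effect.
; Release disables custom depth.
; IA_Hold alternately creates a WB_lHouseInfo popup at the mouse position and removes it, while clicking the actor hides an opened popup.
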(event `self.Capsule.OnInputTouchBegin`
  (params (FingerIndex :type "ETouchIndex Enum" :default "Touch1") (TouchedComponent :type "PrimitiveComponent Object Reference"))
  ;[0 0 0 1 22] set render material
  (`PrimitiveComponent.SetRenderCustomDepth` (`self.1lvlHouse`) true :!label _label)
  (`PrimitiveComponent.SetRenderCustomDepth` (`self.2lvlHouse`) true)
  (`PrimitiveComponent.SetRenderCustomDepth` (`self.3lvlHouse`) true)
  (`PrimitiveComponent.SetRenderCustomDepth` (`self.4lvlHouse`) true)
  (`PrimitiveComponent.SetRenderCustomDepth` (`self.5lvlHouse`) true)
  (`PrimitiveComponent.SetRenderCustomDepth` (`self.6lvlHouse`) true)
  (`PrimitiveComponent.SetRenderCustomDepth` (`self.7lvlHouse`) true)
  (`PrimitiveComponent.SetRenderCustomDepth` (`self.8lvlHouse`) true)
  (`PrimitiveComponent.SetRenderCustomDepth` (`self.9lvlHouse`) true)
  (`PrimitiveComponent.SetRenderCustomDepth` (`self.10lvlHouse`) true)
  (`PrimitiveComponent.SetRenderCustomDepth` (`self.11lvlHouse`) true)
  (`PrimitiveComponent.SetRenderCustomDepth` (`self.12lvlHouse`) true)
  (`PrimitiveComponent.SetRenderCustomDepth` (`self.13lvlHouse`) true)
  (`PrimitiveComponent.SetRenderCustomDepth` (`self.14lvlHouse`) true)
  (`PrimitiveComponent.SetRenderCustomDepth` (`self.15lvlHouse`) true)
  (`PrimitiveComponent.SetRenderCustomDepth` (`self.16lvlHouse`) true)
  (`PrimitiveComponent.SetRenderCustomDepth` (`self.17lvlHouse`) true)
  (`PrimitiveComponent.SetRenderCustomDepth` (`self.18lvlHouse`) true)
  (set `self.IsInteracted` true)
  (bind _foundwidgets (`WidgetBlueprintLibrary.GetAllWidgetsOfClass` "/Game/Widgets/WB_Main.WB_Main_C" false))
  (bind _output_get (set `self.Found Widgets` _foundwidgets))
  (bind _output (`|GetArrayItem` _output_get))
  (set `/Game/Widgets/WB_Main.Money` (+ (`/Game/Widgets/WB_Main.Money` _output) 1.0) _output)
  (`AddComponent|NODE_AddNiagaraComponent-0` :`RelativeTransform` (`KismetMathLibrary.MakeTransform` (0.0 0.0 350.0) (struct :`Pitch` 100.0 :`Yaw` 100.0 :`Roll` 90.0))))

(event `self.Capsule.OnClicked`
  (params (TouchedComponent :type "PrimitiveComponent Object Reference") (ButtonPressed :type "Key Structure"))
  (goto _label))

(event `self.Capsule.OnReleased`
  (params (TouchedComponent :type "PrimitiveComponent Object Reference") (ButtonReleased :type "Key Structure"))
  ;[0 0 0 1 22] set render material
  (`PrimitiveComponent.SetRenderCustomDepth` (`self.1lvlHouse`) false :!label _label_2)
  (`PrimitiveComponent.SetRenderCustomDepth` (`self.2lvlHouse`) false)
  (`PrimitiveComponent.SetRenderCustomDepth` (`self.3lvlHouse`) false)
  (`PrimitiveComponent.SetRenderCustomDepth` (`self.4lvlHouse`) false)
  (`PrimitiveComponent.SetRenderCustomDepth` (`self.5lvlHouse`) false)
  (`PrimitiveComponent.SetRenderCustomDepth` (`self.6lvlHouse`) false)
  (`PrimitiveComponent.SetRenderCustomDepth` (`self.7lvlHouse`) false)
  (`PrimitiveComponent.SetRenderCustomDepth` (`self.8lvlHouse`) false)
  (`PrimitiveComponent.SetRenderCustomDepth` (`self.9lvlHouse`) false)
  (`PrimitiveComponent.SetRenderCustomDepth` (`self.10lvlHouse`) false)
  (`PrimitiveComponent.SetRenderCustomDepth` (`self.11lvlHouse`) false)
  (`PrimitiveComponent.SetRenderCustomDepth` (`self.12lvlHouse`) false)
  (`PrimitiveComponent.SetRenderCustomDepth` (`self.13lvlHouse`) false)
  (`PrimitiveComponent.SetRenderCustomDepth` (`self.14lvlHouse`) false)
  (`PrimitiveComponent.SetRenderCustomDepth` (`self.15lvlHouse`) false)
  (`PrimitiveComponent.SetRenderCustomDepth` (`self.16lvlHouse`) false)
  (`PrimitiveComponent.SetRenderCustomDepth` (`self.17lvlHouse`) false)
  (`PrimitiveComponent.SetRenderCustomDepth` (`self.18lvlHouse`) false))

(event `self.Capsule.OnInputTouchEnd`
  (params (FingerIndex :type "ETouchIndex Enum" :default "Touch1") (TouchedComponent :type "PrimitiveComponent Object Reference"))
  (goto _label_2))

(event `EnhancedInput|/Game/Widgets/controls/IA_Hold`
  (params (ActionValue :type Boolean) (ElapsedSeconds :type "Float (double-precision)") (TriggeredSeconds :type "Float (double-precision)") (InputAction :type "InputAction Object Reference" :default "/Game/Widgets/controls/IA_Hold.IA_Hold"))
  (bind (_locationx _locationy) (`PlayerController.GetMousePosition` (`GameplayStatics.GetPlayerController` 0)))
  (:`Triggered`
    (`/Engine/EditorBlueprintResources/StandardMacros.FlipFlop`
      (:`A`
        (bind _returnvalue (`|CreateWidget` "/Game/Widgets/WB_lHouseInfo.WB_lHouseInfo_C" null (`self.WBClickerRef`)))
        (`UserWidget.AddToViewport` _returnvalue 0)
        (`UserWidget.SetPositionInViewport` _returnvalue (`KismetMathLibrary.MakeVector2D` _locationx _locationy) false)
        (set `self.isWidgetOpened` true))
      (:`B`
        (`Widget.RemoveFromParent` _returnvalue)))))

(event `self.ReceiveActorOnClicked`
  (params (ButtonPressed :type "Key Structure"))
  (if (`self.isWidgetOpened`)
    (`Widget.SetVisibility` (stale `EnhancedInput|/Game/Widgets/controls/IA_Hold` _returnvalue) "Hidden")))

(fn `UserConstructionScript`)