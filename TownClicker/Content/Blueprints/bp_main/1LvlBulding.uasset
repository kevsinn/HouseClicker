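; Clickable level 1 building actor for a clicker game that earns the player money on each tap or click.
; Pressing the capsule turns on the house mesh's custom depth, adds 1 to Money on the first WB_Clicker widget found and adds a Niagara effect above it.
; Releasing turns custom depth off.
; The construction script and CreateWidget function are empty.
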(event `self.Capsule.OnInputTouchBegin`
  (params (FingerIndex :type "ETouchIndex Enum" :default "Touch1") (TouchedComponent :type "PrimitiveComponent Object Reference"))
  (`PrimitiveComponent.SetRenderCustomDepth` (`self.1lvlHouse`) true :!label _label)
  (bind _foundwidgets (`WidgetBlueprintLibrary.GetAllWidgetsOfClass` "/Game/Widgets/WB_Clicker.WB_Clicker_C" false))
  (bind _output_get (set `self.Found Widgets` _foundwidgets))
  (bind _output (`|GetArrayItem` _output_get))
  (set `/Game/Widgets/WB_Clicker.Money` (+ (`/Game/Widgets/WB_Clicker.Money` _output) 1.0) _output)
  (`AddComponent|NODE_AddNiagaraComponent-0` :`RelativeTransform` (`KismetMathLibrary.MakeTransform` (0.0 0.0 200.0) (struct :`Pitch` 100.0 :`Roll` 90.0))))

(event `self.Capsule.OnClicked`
  (params (TouchedComponent :type "PrimitiveComponent Object Reference") (ButtonPressed :type "Key Structure"))
  (goto _label))

(event `self.Capsule.OnReleased`
  (params (TouchedComponent :type "PrimitiveComponent Object Reference") (ButtonReleased :type "Key Structure"))
  (`PrimitiveComponent.SetRenderCustomDepth` (`self.1lvlHouse`) false :!label _label_2))

(event `self.Capsule.OnInputTouchEnd`
  (params (FingerIndex :type "ETouchIndex Enum" :default "Touch1") (TouchedComponent :type "PrimitiveComponent Object Reference"))
  (goto _label_2))

(fn `CreateWidget`
  (returns (Widget :type "/Game/Blueprints/interface/BP_PinBuildingsAmount Interface"))
  (locals (LocalRefWidget :type "Array of UserWidget Object Reference"))
  (return null))

(fn `UserConstructionScript`)